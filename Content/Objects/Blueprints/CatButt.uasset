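; CatButt is a VR pickup actor whose release reveals hidden buildings in the level.
; Pickup, called by BP_MotionController, disables physics and snaps it to the hand mesh's cube socket.
; Drop detaches it without re-enabling physics, unhides Buildings, enables collision on Buildings and TriggerBox, and plays an Enderman teleport sound at a fixed location.
; SetGripType returns a fixed grip type.
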(event `/SteamVRInput/EpicTemplates/VRTemplate/Blueprints/PickupActorInterface.Pickup`
  (params (AttachTo :type "SceneComponent Object Reference") (HandMesh :type "SceneComponent Object Reference") (HandType :type "EControllerHand Enum" :default "Left") (FlipSocket :type Boolean))
  (`PrimitiveComponent.SetSimulatePhysics` (`self.StaticMeshComponent`) false)
  (`SceneComponent.K2_AttachToComponent` (`self.K2_GetRootComponent`) HandMesh "cubeSocket" "SnapToTarget" "SnapToTarget" "KeepWorld" false))

(event `/SteamVRInput/EpicTemplates/VRTemplate/Blueprints/PickupActorInterface.Drop`
  (bind _buildings (`self.buildings`))
  (`self.K2_DetachFromActor` "KeepWorld" "KeepWorld" "KeepWorld")
  (`self.SetActorHiddenInGame` _buildings false)
  (`self.SetActorEnableCollision` _buildings true)
  (`self.SetActorEnableCollision` (`self.trigger_box`) true)
  (`GameplayStatics.SpawnSoundAtLocation` "/Game/Objects/Sounds/Enderman_Teleport_Cue.Enderman_Teleport_Cue" (2.0 0.0 80.0) (struct) 1.3 1.0 0.0 null null))

(fn `SetGripType`
  (returns (SetHandPose :type "/SteamVRInput/Sample/Characters/Hands/HandPoseEnum Enum"))
  (return "NewEnumerator4"))

(fn `UserConstructionScript`)