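; BP_PickupCube is a grabbable cube that remotely drives the position of a separate Target actor.
; Each Tick it remaps its own location from a small hard-coded region into a larger one by offset and uniform scale, clamps it to that region, and moves Target there with sweep.
; Pickup disables mesh physics and attaches the cube to the supplied component; Drop re-enables physics and detaches it, both keeping world transform.
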(event `self.ReceiveTick`
  (params (DeltaSeconds :type "Float (single-precision)"))
  (bind _output_get (set `self.smallMin` (-50.0 10.0 120.0)))
  (bind _output_get_2 (set `self.largeMin` (10.0 -385.0 185.0)))
  (bind _output_get_3 (set `self.largeMax` (385.0 -10.0 560.0)))
  (`self.K2_SetActorLocation` (`self.Target`) (`KismetMathLibrary.MakeVector` (`KismetMathLibrary.FMin` (`KismetMathLibrary.FMax` (.x (+ (* (- (`self.K2_GetActorLocation`) _output_get) (7.5 7.5 7.5)) _output_get_2)) (.x _output_get_2)) (.x _output_get_3)) (`KismetMathLibrary.FMin` (`KismetMathLibrary.FMax` (.y (+ (* (- (`self.K2_GetActorLocation`) _output_get) (7.5 7.5 7.5)) _output_get_2)) (.y _output_get_2)) (.y _output_get_3)) (`KismetMathLibrary.FMin` (`KismetMathLibrary.FMax` (.z (+ (* (- (`self.K2_GetActorLocation`) _output_get) (7.5 7.5 7.5)) _output_get_2)) (.z _output_get_2)) (.z _output_get_3))) true false))

(event `Pickup_1`
  (params (AttachTo :type "SceneComponent Object Reference"))
  (`PrimitiveComponent.SetSimulatePhysics` (`self.StaticMeshComponent`) false)
  (`SceneComponent.K2_AttachToComponent` (`self.K2_GetRootComponent`) AttachTo "None" "KeepWorld" "KeepWorld" "KeepWorld" false))

(event `Drop_1`
  (`PrimitiveComponent.SetSimulatePhysics` (`self.StaticMeshComponent`) true)
  (`self.K2_DetachFromActor` "KeepWorld" "KeepWorld" "KeepWorld"))

(fn `UserConstructionScript`)