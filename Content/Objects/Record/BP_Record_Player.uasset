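; Record player actor whose needle arm follows a separate pointer actor and starts music when dropped over the record.
; Tick computes the yaw toward the pointer and turns the needle while the pointer is picked up.
; Releasing it within a set yaw range plays the Whiteroomed sound once at a fixed location, then spins the record indefinitely by a per-frame step.
; An older, disconnected copy of this logic remains in the graph.
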(event `self.ReceiveTick`
  (params (DeltaSeconds :type "Float (single-precision)"))
  (bind _record_update (`self.record_update`))
  (bind (_returnvalue_roll _returnvalue_pitch _returnvalue_yaw) (`KismetMathLibrary.BreakRotator` (`SceneComponent.K2_GetComponentRotation` _record_update)))
  (bind (_returnvalue_roll_2 _returnvalue_pitch_2 _returnvalue_yaw_2) (`KismetMathLibrary.BreakRotator` (`KismetMathLibrary.MakeRotFromX` (- (`self.K2_GetActorLocation` (`self.NeedlePointerReference`)) (`SceneComponent.K2_GetComponentLocation` (`self.needle`))))))
  (`|ExecutionSequence`
    (:`then_0`
      (set `self.NeedleDirection` _returnvalue_yaw_2))
    (:`then_1`
      (if (`/Game/Objects/Record/BP_NeedlePointer.pickedUp` (`self.NeedlePointerReference`))
        (`SceneComponent.K2_SetWorldRotation` (`self.needle`) (`KismetMathLibrary.MakeRotator` 0.0 0.0 (`self.NeedleDirection`)) false false)))
    (:`then_2`
      (if (and (not (`/Game/Objects/Record/BP_NeedlePointer.pickedUp` (`self.NeedlePointerReference`))) (`KismetMathLibrary.InRange_FloatFloat` (`self.NeedleDirection`) 105.0 165.0))
        (if (not (`self.played`))
          (`GameplayStatics.PlaySoundAtLocation` "/Game/Objects/Record/whiteroomed.whiteroomed" (49.0 -33.5 45.5) (struct) 1.0 1.0 0.0 null null null)
          (set `self.played` true))))
    (:`then_3`
      (if (`self.played`)
        (`SceneComponent.K2_SetWorldRotation` _record_update (`KismetMathLibrary.MakeRotator` 0.0 0.0 (+ _returnvalue_yaw 2.0)) false false)))))

(fn `UserConstructionScript`)